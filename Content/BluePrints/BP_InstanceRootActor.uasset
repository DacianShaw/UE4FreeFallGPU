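; BP_InstanceRootActor is an unfinished actor that sets up render-target-based position and velocity simulation, apparently for instances.
; BeginPlay creates dynamic materials for position update, initialization and velocity update, then clears two position and two velocity render targets, paired as if for ping-ponging.
; Only the position material is stored, as the velocity assignment is disconnected.
; Tick holds an empty sequence, so no simulation step runs.
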(event `self.ReceiveBeginPlay`
  (`|ExecutionSequence`
    (:`then_0`
      (bind _returnvalue (`KismetMaterialLibrary.CreateDynamicMaterialInstance` "/Game/Materials/PositionUpdateMaterial.PositionUpdateMaterial"))
      (set `self.UpdatePosition_Mat` _returnvalue)
      (`KismetMaterialLibrary.CreateDynamicMaterialInstance` "/Game/Materials/InitializeMaterial.InitializeMaterial"))
    (:`then_1`
      (bind _returnvalue_2 (`KismetMaterialLibrary.CreateDynamicMaterialInstance` "/Game/Materials/VelocityUpdateMaterial.VelocityUpdateMaterial")))
    (:`then_2`
      ;[1 1 1] prepare render target
      (`KismetRenderingLibrary.ClearRenderTarget2D` "/Game/Materials/PositionRt1.PositionRt1")
      (`KismetRenderingLibrary.ClearRenderTarget2D` "/Game/Materials/PositionRT2.PositionRT2")
      (`KismetRenderingLibrary.ClearRenderTarget2D` "/Game/Materials/VelocityRT1.VelocityRT1")
      (`KismetRenderingLibrary.ClearRenderTarget2D` "/Game/Materials/VelocityRT2.VelocityRT2"))))

(event `self.ReceiveTick`
  (params (DeltaSeconds :type "Float (single-precision)"))
  (`|ExecutionSequence`))

(fn `UserConstructionScript`)