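; Actor that seeds a position render target and spawns a pool of cube actors, one per texel of a position texture.
; On BeginPlay it creates a dynamic initialization material, feeds it the Range from a parameter collection and draws it into PositionRt1.
; It then spawns one BP_Cube for each pixel of PositionRT and stores them in ActorList.
; Tick is empty, so nothing here moves the cubes.
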(event `self.ReceiveBeginPlay`
  (bind _initialzieposandvelocity_mat (`self.InitialziePosAndVelocity_mat`))
  (bind _positionrt (`self.PositionRT`))
  ;[1 1 1] initialization
  (`|ExecutionSequence`
    (:`then_0`
      (bind _returnvalue (`KismetMaterialLibrary.CreateDynamicMaterialInstance` "/Game/Materials/InitializeMaterial.InitializeMaterial"))
      (set `self.InitialziePosAndVelocity_mat` _returnvalue))
    (:`then_1`
      (bind _returnvalue_2 (`KismetMaterialLibrary.GetScalarParameterValue` "/Game/Materials/ParametersCollection.ParametersCollection" "Range"))
      (`MaterialInstanceDynamic.SetScalarParameterValue` _initialzieposandvelocity_mat "Range" _returnvalue_2)
      (`KismetRenderingLibrary.DrawMaterialToRenderTarget` "/Game/Materials/PositionRt1.PositionRt1" _initialzieposandvelocity_mat)
      (set `self.Range` _returnvalue_2)
      (`MaterialInstanceDynamic.SetScalarParameterValue` _initialzieposandvelocity_mat "Range" 2.0))
    (:`then_2`
      (for _ (range (* (`TextureRenderTarget2D.SizeX` _positionrt) (`TextureRenderTarget2D.SizeY` _positionrt)))
        (bind _returnvalue_3 (`|SpawnActorFromClass` "/Game/BluePrints/BP_Cube.BP_Cube_C" (`KismetMathLibrary.MakeTransform` (0.0 0.0 0.0)) "Undefined" "OverrideRootScale" null null))
        (`KismetArrayLibrary.Array_Add` (`self.actorList`) _returnvalue_3)))))

(fn `UserConstructionScript`)